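; Spawner actor that builds an endless chain of BP_PlatformActor platforms along the X axis.
; On BeginPlay it places a start block at a random height, then spawns the next after a short delay.
; Each new block is offset from the last by its tile width plus a random gap, with clamped height variation.
; Non-start platforms entering Trigger_Box each spawn one successor, guarded by a per-platform flag.
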(event `self.ReceiveBeginPlay`
  (bind _returnvalue (`|SpawnActorFromClass` "/Game/Blueprints/BP_PlatformActor.BP_PlatformActor_C" (`KismetMathLibrary.MakeTransform` (`KismetMathLibrary.MakeVector` 0.0 0.0 (`KismetMathLibrary.RandomFloatInRange` -350.0 -200.0)) (struct) (1.0 1.0 1.0)) "AdjustIfPossibleButDontSpawnIfColliding" "OverrideRootScale" null true))
  (set `self.LastSpawnedBlock_Ref` _returnvalue)
  (`KismetSystemLibrary.Delay` 0.5)
  (`self.SpawnNextBlock`))

(event `SpawnNextBlock`
  (bind _lastspawnedblock_ref (`self.LastSpawnedBlock_Ref`))
  (bind (_returnvalue_x _returnvalue_y _returnvalue_z) (`KismetMathLibrary.BreakVector` (`self.K2_GetActorLocation` (`self.LastSpawnedBlock_Ref`))))
  (bind _returnvalue_x_2 (`KismetMathLibrary.BreakVector` (`self.K2_GetActorLocation` _lastspawnedblock_ref)))
  (bind _returnvalue (`|SpawnActorFromClass` "/Game/Blueprints/BP_PlatformActor.BP_PlatformActor_C" (`KismetMathLibrary.MakeTransform` (`KismetMathLibrary.MakeVector` (+ (+ (* (`/Game/Blueprints/BP_PlatformActor.HorTiles` _lastspawnedblock_ref) 200.0) _returnvalue_x_2) (`KismetMathLibrary.RandomFloatInRange` 300.0 400.0)) 0.0 (`KismetMathLibrary.FClamp` (+ _returnvalue_z (`KismetMathLibrary.RandomFloatInRange` -120.0 120.0)) -400.0 200.0))) "AdjustIfPossibleButDontSpawnIfColliding" "OverrideRootScale"))
  (set `self.LastSpawnedBlock_Ref` _returnvalue))

(event `self.Trigger_Box.OnComponentBeginOverlap`
  (params (OverlappedComponent :type "PrimitiveComponent Object Reference") (OtherActor :type "Actor Object Reference") (OtherComp :type "PrimitiveComponent Object Reference") (OtherBodyIndex :type Integer) (bFromSweep :type Boolean) (SweepResult :type "HitResult Structure (by ref)"))
  (bind _asbp_platform_actor (cast `/Game/Blueprints/BP_PlatformActor` OtherActor))
  (if (`/Game/Blueprints/BP_PlatformActor.StartBlock?` _asbp_platform_actor)
    _
    (elif (not (`/Game/Blueprints/BP_PlatformActor.NextBlockSpawned?` _asbp_platform_actor))
      (set `/Game/Blueprints/BP_PlatformActor.NextBlockSpawned?` true _asbp_platform_actor)
      (`self.SpawnNextBlock`))))

(fn `UserConstructionScript`)