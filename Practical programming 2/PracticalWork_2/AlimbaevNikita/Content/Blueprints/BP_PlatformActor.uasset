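; BP_PlatformActor is a side-scrolling platform segment that constantly moves along negative X and awards score when the main character reaches it.
; BeginPlay builds a row of randomly chosen brace sprites, long for a start block and short, random-length otherwise.
; Regular segments randomly place a hazard and set a trigger on the last tile, while start blocks destroy both.
; That trigger adds the tile count to the GameMode score once, if the character is alive.
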(event `self.ReceiveBeginPlay`
  ;[1 1 1] Begin Play Event
  (`|ExecutionSequence`
    (:`then_0`
      (set `self.HorTiles` (select `bool` (`self.StartBlock?`) :`false` (`KismetMathLibrary.RandomIntegerInRange` 4 6) :`true` 15))
      (for _index (range (`self.HorTiles`))
        (bind _returnvalue (`AddComponent|NODE_AddPaperSpriteComponent-0` :`RelativeTransform` (`KismetMathLibrary.MakeTransform` (`KismetMathLibrary.MakeVector` (* _index 200.0)))))
        (`PaperSpriteComponent.SetSprite` _returnvalue (select `bool` (`KismetMathLibrary.RandomBool`) :`false` "/Game/Assets/Sprites/Platform/Brace_001_Sprite.Brace_001_Sprite" :`true` "/Game/Assets/Sprites/Platform/Brace_007_Sprite.Brace_007_Sprite" :!type "PaperSprite Object Reference"))))
    (:`then_1`
      (if (`self.StartBlock?`)
        (`ActorComponent.K2_DestroyComponent` (`self.ScoreTrigger_Box`))
        (`ActorComponent.K2_DestroyComponent` (`self.Hazard`))
        (else
          (`SceneComponent.K2_SetRelativeLocation` (`self.Hazard`) (`KismetMathLibrary.MakeVector` (* (`KismetMathLibrary.RandomIntegerInRange` 0 (- (`self.HorTiles`) 1)) 200.0) 0.0 0.0) false false)
          (`SceneComponent.K2_SetRelativeLocation` (`self.ScoreTrigger_Box`) (`KismetMathLibrary.MakeVector` (* (- (`self.HorTiles`) 1) 200.0)) false false))))))

(event `self.ReceiveTick`
  (params (DeltaSeconds :type "Float (single-precision)"))
  (`self.K2_AddActorWorldOffset` (`KismetMathLibrary.MakeVector` (* DeltaSeconds -900.0))))

(event `self.ScoreTrigger_Box.OnComponentBeginOverlap`
  (params (OverlappedComponent :type "PrimitiveComponent Object Reference") (OtherActor :type "Actor Object Reference") (OtherComp :type "PrimitiveComponent Object Reference") (OtherBodyIndex :type Integer) (bFromSweep :type Boolean) (SweepResult :type "HitResult Structure (by ref)"))
  (bind _asbp_main_character (cast `/Game/Blueprints/BP_MainCharacter` OtherActor))
  (if (and (not (`/Game/Blueprints/BP_MainCharacter.Is Dead ?` _asbp_main_character)) (not (`self.StartBlock?`)))
    (`/Engine/EditorBlueprintResources/StandardMacros.DoOnce` false
      (:`Completed`
        (bind _asbp_game_mode (cast `/Game/Blueprints/BP_GameMode` (`GameplayStatics.GetGameMode`)))
        (`/Game/Blueprints/BP_GameMode.UpdateScore` _asbp_game_mode (`self.HorTiles`))))))

(fn `UserConstructionScript`)