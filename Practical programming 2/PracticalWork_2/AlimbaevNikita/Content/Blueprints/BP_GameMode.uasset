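; BP_GameMode is the game mode that tracks the current score and a persistent best score, and drives the in-game HUD and game-over screen.
; On BeginPlay it loads or creates a ScoreSaveGame_BP in a save slot, then creates the WG_InGame widget showing both scores.
; UpdateScore adds points and refreshes the HUD.
; GameOver saves any new high score, shows the mouse cursor and opens WG_GameOver.
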(event `self.ReceiveBeginPlay`
  (`self.CheckSaveScore`)
  (bind _returnvalue (`|CreateWidget` "/Game/Blueprints/WG_InGame.WG_InGame_C" (`GameplayStatics.GetPlayerController` 0)))
  (bind _output_get (set `self.Game HUD Reference` _returnvalue))
  (`UserWidget.AddToViewport` _output_get 1)
  (`/Game/Blueprints/WG_InGame.Update Scores` (`self.Game HUD Reference`) (`self.Score`) (`self.Best Score`)))

(event `CheckSaveScore`
  ;[1 1 1] Проверьте, существует ли слот SaveGame "HS"
  (bind _returnvalue (`GameplayStatics.DoesSaveGameExist` "DefaultSlot"))
  (if _returnvalue
    (bind _returnvalue_2 (`GameplayStatics.LoadGameFromSlot` "DefaultSlot"))
    (bind _asscore_save_game_bp (cast `/Game/Blueprints/ScoreSaveGame_BP` _returnvalue_2))
    (bind _output_get (set `self.High SaveGame Reference` _asscore_save_game_bp))
    (set `self.Best Score` (`/Game/Blueprints/ScoreSaveGame_BP.HighScore` _output_get))
    (else
      (bind _returnvalue_3 (`GameplayStatics.CreateSaveGameObject` "/Game/Blueprints/ScoreSaveGame_BP.ScoreSaveGame_BP_C"))
      (bind _asscore_save_game_bp_2 (cast `/Game/Blueprints/ScoreSaveGame_BP` _returnvalue_3))
      (bind _output_get_2 (set `self.High SaveGame Reference` _asscore_save_game_bp_2))
      (bind _output_get_3 (set `/Game/Blueprints/ScoreSaveGame_BP.HighScore` 0 _output_get_2))
      (set `self.Best Score` _output_get_3)
      (`GameplayStatics.SaveGameToSlot` _output_get_2 "DefaultSlot")))
  (set `self.Score` 0))

(event `UpdateHighScore`
  (bind _high_savegame_reference (`self.High SaveGame Reference`))
  ;[1 1 1] Обновление HighScore
  (if (> (`self.Score`) (`self.Best Score`))
    (bind _output_get (set `self.Best Score` (`self.Score`)))
    (set `/Game/Blueprints/ScoreSaveGame_BP.HighScore` _output_get _high_savegame_reference)
    (`GameplayStatics.SaveGameToSlot` _high_savegame_reference "DefaultSlot")))

(event `UpdateScore`
  (params (value :type Integer))
  ;[1 1 1] Update Score
  (set `self.Score` (+ value (`self.Score`)))
  (`/Game/Blueprints/WG_InGame.Update Scores` (`self.Game HUD Reference`) (`self.Score`) (`self.Best Score`)))

(event `GameOver`
  (bind _returnvalue (`GameplayStatics.GetPlayerController` 0))
  (`self.UpdateHighScore`)
  (`/Game/Blueprints/WG_InGame.Update Scores` (`self.Game HUD Reference`) (`self.Score`) (`self.Best Score`))
  (set `PlayerController.bShowMouseCursor` true _returnvalue)
  (bind _returnvalue_2 (`|CreateWidget` "/Game/Blueprints/WG_GameOver.WG_GameOver_C" _returnvalue))
  (bind _output_get (set `self.GameOver Widget Reference` _returnvalue_2))
  (`UserWidget.AddToViewport` _output_get 0))

(fn `UserConstructionScript`)