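; Paper2D player character with jump, double jump and a death sequence that ends the game.
; Touch events and the Jump action share one routine: a normal jump on the ground, then one launch in midair.
; Tick picks the run, jump or fall flipbook from movement state.
; DeathSequence disables collision, flings and rotates the sprite via timeline, calls BP_GameMode's GameOver after a delay, and later halts movement in flying mode.
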(event `DeathSequence`
  (bind _charactermovement (`self.CharacterMovement`))
  ;[1 1 1] Death Sequence
  (if (not (`self.Is Dead ?`))
    (`|ExecutionSequence`
      (:`then_0`
        (set `self.Is Dead ?` true)
        (`self.SetActorEnableCollision` false)
        (`self.LaunchCharacter` (0.0 0.0 2500.0) true true)
        (bind (_direction _pitchvalue) (`Timeline|RotationTimeline`)
          (:`Update`
            (`SceneComponent.K2_SetRelativeRotation` (`self.Sprite`) (`KismetMathLibrary.MakeRotator` 0.0 _pitchvalue) false false))))
      (:`then_1`
        (`KismetSystemLibrary.Delay` 1.0)
        (bind _asbp_game_mode (cast `/Game/Blueprints/BP_GameMode` (`GameplayStatics.GetGameMode`)))
        (`/Game/Blueprints/BP_GameMode.GameOver` _asbp_game_mode))
      (:`then_2`
        (`KismetSystemLibrary.Delay` 3.0)
        (`CharacterMovementComponent.SetMovementMode` _charactermovement "MOVE_Flying" 0)
        (`MovementComponent.StopMovementImmediately` _charactermovement)))))

(event `self.ReceiveBeginPlay`
  ;[1 1 1] Begin Play(Initialization)
  (set `self.Is Dead ?` false)
  (set `self.Can Double Jump` false))

(event `UpdateAnimation`
  (bind (_velocity_x _velocity_y _velocity_z) (`KismetMathLibrary.BreakVector` (`MovementComponent.Velocity` (`self.CharacterMovement`))))
  ;[1 1 1] Update Player Animation
  (if (`self.Is Dead ?`)
    (set `self.Player Animation` "/Game/Assets/Flipbooks/Fall_Flipbook.Fall_Flipbook")
    (elif (`NavMovementComponent.IsMovingOnGround` (`self.CharacterMovement`))
      (set `self.Player Animation` "/Game/Assets/Flipbooks/Run_Flipbook.Run_Flipbook")
      (else
        (set `self.Player Animation` (select `bool` (< _velocity_z 0.0) :`false` "/Game/Assets/Flipbooks/Jump_Flipbook.Jump_Flipbook" :`true` "/Game/Assets/Flipbooks/Fall_Flipbook.Fall_Flipbook" :!type "PaperFlipbook Object Reference")))))
  (`PaperFlipbookComponent.SetFlipbook` (`self.Sprite`) (`self.Player Animation`)))

(event `self.ReceiveTick`
  (params (DeltaSeconds :type "Float (single-precision)"))
  ;[1 1 1] Tick Event
  (`self.UpdateAnimation`))

(event `self.ReceiveActorOnInputTouchBegin`
  (params (FingerIndex :type "ETouchIndex Enum" :default "Touch1"))
  ;[1 1 1] Прыжок
  (if (not (`self.Is Dead ?`)) :!label _label
    (if (`NavMovementComponent.IsMovingOnGround` (`self.CharacterMovement`))
      (`self.Jump`)
      (set `self.Can Double Jump` true)
      (elif (`self.Can Double Jump`)
        (`self.LaunchCharacter` (0.0 0.0 1200.0) false true)
        (set `self.Can Double Jump` false)))))

(event `InputAction|Jump`
  (params (Key :type "Key Structure"))
  ;[1 1 1] Прыжок
  (:`Pressed`
    (goto _label)))

(event `InputTouch`
  (params (Location :type "Vector Structure") (FingerIndex :type "ETouchIndex Enum"))
  ;[1 1 1] Прыжок
  (:`Released`
    (goto _label)))

(fn `UserConstructionScript`)